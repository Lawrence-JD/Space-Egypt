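; AI controller for Roomba enemies that runs the BT_RoombaProto behavior tree and feeds its blackboard.
; Perception updates set whether it can see the player.
; Tick polls player and Roomba vessels for held light, counts down the Roomba's light-taken cooldown, and writes both results as flags.
; Tick also advances through the pawn's spline path points when within range, looping, and publishes the current one as the patrol target.
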(event OnTargetPerceptionUpdated(AIPerception)
  (params (Actor :type Actor%20Object%20Reference) (Stimulus :type AI%20Stimulus%20Structure))
  ;[1 1 1] Can See Player Code
  (Utilities|Casting|CastToSpeegyptPlayer Actor)
  (AI|Components|Blackboard|SetValueasBool (AI|GetBlackboard 0) (Utilities|Name|MakeLiteralName "CanSeePlayer") (.bSuccessfullySensed (Utilities|Struct|BreakAIStimulus Stimulus))))

(event EventBeginPlay
  (Utilities|FlowControl|Sequence
    (:then_0
      (bind _asroomba_base (Utilities|Casting|CastToRoombaBase (Pawn|GetControlledPawn)))
      (bind _output_get (Variables|Default|SetSplinePath (Variables|/Script/Speegypt.RoombaBase|GetPath _asroomba_base)))
      (Variables|Default|SetCurrentSplineNodeLocation (Spline|GetLocationatSplinePoint _output_get 0 "World")))
    (:then_1
      (AI|RunBehaviorTree "/Game/Speegypt/Core/AI/Roomba/BT_RoombaProto.BT_RoombaProto"))))

(event EventTick
  (params (DeltaSeconds :type Float%20%28single-precision%29))
  (Utilities|FlowControl|Sequence
    (:then_0
      ;[1 0 0] Change to use dispatcher (Player/Roomba Has Light Code)
      (bind _asspeegypt_player (Utilities|Casting|CastToSpeegyptPlayer (Game|GetPlayerCharacter 0)))
      (bind _returnvalue (Class|Vessel|GetVesselState (Variables|/Script/Speegypt.SpeegyptCharacter|GetRightVessel _asspeegypt_player)))
      (AI|Components|Blackboard|SetValueasBool (AI|GetBlackboard 0) (Utilities|Name|MakeLiteralName "PlayerHasLight") (not (Utilities|Enum|Equal(Enum) _returnvalue "Empty"))))
    (:then_1
      (bind _asroomba_base (Utilities|Casting|CastToRoombaBase (Pawn|GetControlledPawn)))
      (bind _returnvalue_2 (Class|Vessel|GetVesselState (Variables|/Script/Speegypt.RoombaBase|GetVessel _asroomba_base)))
      (AI|Components|Blackboard|SetValueasBool (AI|GetBlackboard 0) (Utilities|Name|MakeLiteralName "RoombaHasLight") (not (Utilities|Enum|Equal(Enum) _returnvalue_2 "Empty"))))
    (:then_2
      ;[1 1 1] Spline Path Code
      (if (< (Math|Vector|VectorLengthSquared (- (Variables|Default|GetCurrentSplineNodeLocation) (Transformation|GetActorLocation (Pawn|GetControlledPawn)))) (* 1e+02 1e+02))
        (if (> (+ (Variables|Default|GetCurrentSplineNode) 1) (Spline|GetNumberOfSplinePoints (Variables|Default|GetSplinePath)))
          (Variables|Default|SetCurrentSplineNode 0)
          (else
            (Variables|Default|SetCurrentSplineNode (+ (Variables|Default|GetCurrentSplineNode) 1))))
        (Variables|Default|SetCurrentSplineNodeLocation (Spline|GetLocationatSplinePoint (Variables|Default|GetSplinePath) (Variables|Default|GetCurrentSplineNode) "World"))))
    (:then_3
      ;[1 1 1] Take Light Cooldown Code
      (bind _asroomba_base_2 (Utilities|Casting|CastToRoombaBase (Pawn|GetControlledPawn)))
      (if (> (Variables|/Script/Speegypt.RoombaBase|GetLightCooldown _asroomba_base_2) 0.0)
        (Variables|/Script/Speegypt.RoombaBase|SetLightCooldown _asroomba_base_2 (- (Variables|/Script/Speegypt.RoombaBase|GetLightCooldown _asroomba_base_2) DeltaSeconds)))
      (AI|Components|Blackboard|SetValueasBool (AI|GetBlackboard 0) (Utilities|Name|MakeLiteralName "LightTakenRecently") (> (Variables|/Script/Speegypt.RoombaBase|GetLightCooldown _asroomba_base_2) 0.0)))
    (:then_4
      (AI|Components|Blackboard|SetValueasVector (AI|GetBlackboard 0) (Utilities|Name|MakeLiteralName "PathLocation") (Variables|Default|GetCurrentSplineNodeLocation)))))

(fn ConstructionScript)