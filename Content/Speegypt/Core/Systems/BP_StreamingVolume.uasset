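; BP_StreamingVolume is a trigger volume that streams a named level in and out around the player, preserving its state in a save slot.
; Entering loads the level with blocking, then restores its saved data after a delay; leaving saves it, then unloads after a delay.
; A delayed BeginPlay check restores saved data if the player starts inside, otherwise unloads the level.
; The construction script assigns an SGUID; SaveLevel and LoadLevel events are empty.
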(event Custom|Load%20Level)

(event Custom|Save%20Level)

(event Collision|EventActorBeginOverlap
  (params (OtherActor :type Actor%20Object%20Reference))
  (bind _level_name (Variables|Default|GetLevel%20Name))
  (if (== OtherActor (Game|GetPlayerCharacter 0))
    (Game|LoadStreamLevel(byName) (Variables|Default|GetLevel%20Name) true true)
    (Utilities|FlowControl|Delay 1.0)
    (bind _returnvalue (Class|Savior3|NewSlotInstance (Variables|Default|GetSaveSlot))
      (:Success
        (Class|Savior3|LoadLevel _returnvalue _level_name
          (:Success
            (Development|PrintString (Utilities|String|Append (Utilities|String|ToString(Name) _level_name) "Loaded"))))))))

(event Collision|EventActorEndOverlap
  (params (OtherActor :type Actor%20Object%20Reference))
  (bind _level_name (Variables|Default|GetLevel%20Name))
  (if (== OtherActor (Game|GetPlayerCharacter 0))
    (bind _returnvalue (Class|Savior3|NewSlotInstance (Variables|Default|GetSaveSlot))
      (:Success
        (Class|Savior3|SaveLevel _returnvalue _level_name
          (:Success
            (Development|PrintString (Utilities|String|Append (Utilities|String|ToString(Name) _level_name) "SAves"))
            (Utilities|FlowControl|Delay 1.0)
            (Game|UnloadStreamLevel(byName) _level_name false)))))))

(event EventBeginPlay
  (bind _level_name (Variables|Default|GetLevel%20Name))
  (Utilities|FlowControl|Delay 1.0)
  (if (Collision|IsOverlappingActor (Game|GetPlayerCharacter 0) :!class /Script/Engine.Actor)
    (bind _returnvalue (Class|Savior3|NewSlotInstance (Variables|Default|GetSaveSlot))
      (:Success
        (Class|Savior3|LoadLevel _returnvalue _level_name)))
    (else
      (Game|UnloadStreamLevel(byName) _level_name false))))

(fn ConstructionScript
  (Variables|Default|SetSGUID (Class|Savior3|CreateSGUID)))