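; BP_InteractDoor is an interactable door that raises its Cube on a timeline when its conditions allow.
; OnInteract opens it if its MagentaTarget reports fixed or its BeaconSlot holds a beacon, depending on the NeedsFixing and NeedsSlottedBeacon flags, or directly when neither applies.
; A DoOnce blocks retriggering until the timeline finishes and resets it; there is no closing path.
; The construction script initializes MagentaTarget when needed and creates an SGUID.
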(event Custom|Reset
  (bind _startlocation (Variables|Default|GetStartLocation))
  (bind (_x _y _z) (Math|Vector|BreakVector _startlocation))
  (Utilities|FlowControl|DoOnce false) ; enters at Reset
)

(event EventOnInteract
  (params (Player :type Speegypt%20Character%20Object%20Reference))
  (bind _startlocation (Variables|Default|GetStartLocation))
  (bind _magentatarget (Variables|Default|GetMagentaTarget))
  (bind _beaconslot (Variables|Default|GetBeaconSlot))
  (bind (_x _y _z) (Math|Vector|BreakVector _startlocation))
  (Utilities|FlowControl|Sequence
    (:then_0
      (if (Variables|Default|GetNeedsFixing)
        (Utilities|IsValid _magentatarget
          (:Is%20Valid
            (bind _returnvalue (Class|PassiveVesselTarget|GetDataOfComponent _magentatarget (Variables|Default|GetCube)))
            (bind _asmagenta_target_data (Utilities|Casting|CastToMagentaTargetData _returnvalue))
            (if (Variables|/Script/Speegypt.MagentaTargetData|GetbIsFixed _asmagenta_target_data)
              (Utilities|FlowControl|DoOnce false :!label _label
                (:Completed
                  (bind _newtrack_0 (Timeline|openDoor PlayFromStart)
                    (:Update
                      (Transformation|SetWorldLocation (Variables|Default|GetCube) (Math|Vector|MakeVector _x _y (+ _z (* _newtrack_0 3e+02))) false false)
                      (if (!= _newtrack_0 0.0)
                        (Variables|Default|SetisOpen true)
                        (else
                          (Variables|Default|SetisOpen true))))
                    (:Finished
                      (CallFunction|Reset)))))))
          (:Is%20Not%20Valid
            (Development|PrintString "Something is Wrong")))
        (elif (not (Variables|Default|GetNeedsSlottedBeacon))
          (goto _label))))
    (:then_1
      (if (Variables|Default|GetNeedsSlottedBeacon)
        (Utilities|IsValid _beaconslot
          (:Is%20Valid
            (bind _returnvalue_2 (Class|PhysicsBeaconSlot|GetAttachedBeacon _beaconslot))
            (Utilities|IsValid _returnvalue_2
              (:Is%20Valid
                (goto _label)))))))))

(event EventBeginPlay
  (Variables|Default|SetStartLocation (Transformation|GetWorldLocation (Variables|Default|GetCube))))

(fn ConstructionScript
  (Utilities|FlowControl|Sequence
    (:then_0
      (if (Variables|Default|GetNeedsFixing)
        (Class|MagentaVesselTarget|Init (Variables|Default|GetMagentaTarget))))
    (:then_1
      (Variables|Default|SetSGUID (Class|Savior3|CreateSGUID)))))